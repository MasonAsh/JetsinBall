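; BP_Ball is the ball actor for JetsinBall, which can be captured onto a socket of another component and released again.
; Capture turns off physics and collision, teleports the ball to the named socket, attaches it there and sets the Captured flag.
; Release restores physics and collision, clears the flag and detaches the mesh while keeping its world transform.
; The event graph and construction script are empty.
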(fn `Capture`
  (params (AttachTo :type "SceneComponent Object Reference") (Socket :type String))
  (bind _returnvalue (`KismetStringLibrary.Conv_StringToName` Socket))
  (`PrimitiveComponent.SetSimulatePhysics` (`self.StaticMeshComponent`) false)
  (`PrimitiveComponent.SetCollisionEnabled` (`self.StaticMeshComponent`) "NoCollision")
  (`self.K2_SetActorLocation` (`SceneComponent.GetSocketLocation` AttachTo _returnvalue) false true)
  (`self.K2_AttachToComponent` AttachTo _returnvalue "KeepWorld" "KeepWorld" "KeepWorld" false)
  (set `self.captured` true))

(fn `Release`
  (`PrimitiveComponent.SetSimulatePhysics` (`self.StaticMeshComponent`) true)
  (`PrimitiveComponent.SetCollisionEnabled` (`self.StaticMeshComponent`) "QueryAndPhysics")
  (set `self.captured` false)
  (`SceneComponent.K2_DetachFromComponent` (`self.StaticMeshComponent`) "KeepWorld" "KeepWorld" "KeepRelative" true))

(fn `UserConstructionScript`)