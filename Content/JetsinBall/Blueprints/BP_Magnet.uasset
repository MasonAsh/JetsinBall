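; BP_Magnet is a magnet actor that pulls overlapping balls toward itself in JetsinBall.
; Overlapping balls join a list and start a looping timer, roughly 30 Hz, that replaces Tick.
; Each timer tick applies an impulse toward the magnet, scaled by Strength and timer elapsed time, independent of distance.
; Balls are dropped when captured or leaving overlap, and the timer pauses once the list empties.
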(event `self.ReceiveActorBeginOverlap`
  (params (OtherActor :type "Actor Object Reference"))
  (bind _ball (`/Game/JetsinBall/Blueprints/Utilities.IfBall` OtherActor))
  (`KismetArrayLibrary.Array_Add` (`self.Balls`) _ball)
  (bind _returnvalue (`KismetSystemLibrary.K2_SetTimerDelegate` (delegate `MagnetTick`) 0.033333 true))
  (bind _output_get (set `self.MagnetismTimer` _returnvalue))
  (bind _asstatic_mesh_actor (cast `StaticMeshActor` _ball)))

(event `MagnetTick`
  (`self.Magnetism` (stale `self.ReceiveActorBeginOverlap` _asstatic_mesh_actor) (`KismetSystemLibrary.K2_GetTimerElapsedTimeHandle` (stale `self.ReceiveActorBeginOverlap` _output_get))))

(event `self.ReceiveTick`
  (params (DeltaSeconds :type "Float (single-precision)")))

(event `self.ReceiveActorEndOverlap`
  (params (OtherActor :type "Actor Object Reference"))
  (`self.Stop Magnetism` OtherActor))

(fn `Magnetism`
  (params (actor :type "StaticMeshActor Object Reference") (deltaSeconds :type "Float (double-precision)"))
  (for _array_element (`self.Balls`)
    (bind _asbp_ball (cast `/Game/JetsinBall/Ball/BP_Ball` _array_element))
    (if (`/Game/JetsinBall/Ball/BP_Ball.captured` _asbp_ball)
      (`self.Stop Magnetism` _array_element)
      (else
        (bind _asstatic_mesh_actor (cast `StaticMeshActor` _array_element))
        (bind _staticmeshcomponent (`StaticMeshActor.StaticMeshComponent` _asstatic_mesh_actor))
        (bind _returnvalue (- (`self.K2_GetActorLocation`) (`SceneComponent.K2_GetComponentLocation` _staticmeshcomponent)))
        (`PrimitiveComponent.AddImpulse` _staticmeshcomponent (* (* (/ _returnvalue (`KismetMathLibrary.VSize` _returnvalue)) (`self.Strength`)) deltaSeconds) "None" false)))))

(fn `Stop Magnetism`
  (params (Ball :type "Actor Object Reference"))
  (bind _balls (`self.Balls`))
  (bind _asbp_ball (cast `/Game/JetsinBall/Ball/BP_Ball` Ball))
  (`KismetArrayLibrary.Array_RemoveItem` _balls _asbp_ball)
  (if (== (`KismetArrayLibrary.Array_Length` _balls) 0)
    (`KismetSystemLibrary.K2_PauseTimerHandle` (`self.MagnetismTimer`))))

(fn `UserConstructionScript`)